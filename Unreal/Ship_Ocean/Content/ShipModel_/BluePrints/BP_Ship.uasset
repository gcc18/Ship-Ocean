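; BP_Ship is a ship actor built to move its ShipModel along a Spline component.
; A timeline's T value, scaled by spline length, samples local location and rotation, with the root's world position added to the location.
; Each update sets the model's world transform without sweeping and offsets yaw by 90 degrees, ignoring root rotation.
; No event in the graph starts the timeline, and the construction script is empty.
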(fn ConstructionScript)